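; Door Blueprint that swings open or closed on the Q key, with a construction-time option to start open.
; A looping timer, limited to once per frame, steps an alpha that lerps the door's yaw toward OpenRotation or back, making speed frame-rate dependent.
; The timer pauses and flips IsOpen at either end; pressing Q resumes it, or reverses direction mid-swing.
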(event `Key|Q`
  (params (Key :type "Key Structure"))
  (:`Pressed`
    (if (`KismetSystemLibrary.K2_IsValidTimerHandle` (`self.RotateTimerHandle`))
      (if (`KismetSystemLibrary.K2_IsTimerActiveHandle` (`self.RotateTimerHandle`))
        (set `self.IsOpen` (not (`self.IsOpen`)))
        (else
          (`KismetSystemLibrary.K2_UnPauseTimerHandle` (`self.RotateTimerHandle`))))
      (else
        (bind _returnvalue (`KismetSystemLibrary.K2_SetTimerDelegate` (delegate `Rotate`) 0.001 true true))
        (set `self.RotateTimerHandle` _returnvalue)))))

(event `Rotate`
  (bind _alphaalgo (`self.Alphaalgo`))
  (bind _output_get (set `self.Alphaalgo` (`KismetMathLibrary.SelectFloat` (- _alphaalgo 0.005) (+ _alphaalgo 0.005) (`self.IsOpen`))))
  (`SceneComponent.K2_SetRelativeRotation` (`self.Door`) (`KismetMathLibrary.MakeRotator` 0.0 0.0 (`KismetMathLibrary.Lerp` 90.0 (`self.OpenRotation`) _output_get)) false false)
  (if (select `bool` (`self.IsOpen`) :`false` (>= (`self.Alphaalgo`) 1.0) :`true` (<= (`self.Alphaalgo`) 0.0))
    (`KismetSystemLibrary.K2_PauseTimerHandle` (`self.RotateTimerHandle`))
    (set `self.IsOpen` (not (`self.IsOpen`)))))

(fn `UserConstructionScript`
  (bind _output_get (set `self.IsOpen` (`self.StartOpen`)))
  (if _output_get
    (`SceneComponent.K2_SetRelativeRotation` (`self.Door`) (`KismetMathLibrary.MakeRotator` 0.0 0.0 (`self.OpenRotation`)) false false)
    (set `self.Alphaalgo` 1.0)))