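; Tower defense turret that damages pawns in a line toward its target, with a flamethrower particle effect.
; Shoot yaws the turret toward the first enemy in range, with an offset, then runs a multi capsule trace to it and applies damage to every pawn hit.
; EnemyEnter and EnemyExit overrides switch the flame effect on and off when the parent implementation returns true.
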(event `self.Shoot`
  (bind _returnvalue (`SceneComponent.K2_GetComponentLocation` (`self.Torretica`)))
  (bind _returnvalue_2 (`SceneComponent.K2_GetComponentLocation` (`Character.CapsuleComponent` (`|GetArrayItem` (`self.EnemiesInRange`)))))
  (bind (_returnvalue_roll _returnvalue_pitch _returnvalue_yaw) (`KismetMathLibrary.BreakRotator` (`KismetMathLibrary.ComposeRotators` (`KismetMathLibrary.FindLookAtRotation` _returnvalue _returnvalue_2) (struct :`Yaw` 90.0))))
  (`SceneComponent.K2_SetWorldRotation` (`self.Torretica`) (`KismetMathLibrary.MakeRotator` 0.0 0.0 _returnvalue_yaw) false false)
  (bind _outhits (`KismetSystemLibrary.CapsuleTraceMultiForObjects` _returnvalue _returnvalue_2 30.0 20.0 (`|MakeArray` "ObjectTypeQuery3" :!type "EObjectTypeQuery Enum")))
  (for _array_element _outhits
    (`GameplayStatics.ApplyDamage` (`.HitActor` (`GameplayStatics.BreakHitResult` _array_element)) (`self.Damage`) null self "/Script/Engine.DamageType")))

(fn `EnemyEnter`
  (params (Object :type "Object Object Reference"))
  (bind _valid (`parent.EnemyEnter` Object))
  (if _valid
    (`ActorComponent.SetActive` (`self.NS_Projectile_FlameThrower_02`) true false)))

(fn `EnemyExit`
  (params (Object :type "Object Object Reference"))
  (bind _empty (`parent.EnemyExit` Object))
  (if _empty
    (`ActorComponent.SetActive` (`self.NS_Projectile_FlameThrower_02`) false false)))

(fn `UserConstructionScript`)