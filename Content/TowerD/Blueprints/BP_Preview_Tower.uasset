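; BP_Preview_Tower is a tower preview actor that shows by color whether it overlaps obstacles, likely for tower placement.
; The Construction Script applies the Mesh variable to its StaticMesh.
; Overlapping actors tagged "obstaculo" join TowerInRange and turn the material red; end overlap removes them, restoring green once the list is empty.
; Tick prints the tracked actors' names on screen as debug output.
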(event `self.ReceiveBeginPlay`)

(event `self.ReceiveTick`
  (params (DeltaSeconds :type "Float (single-precision)"))
  (for _array_element (`self.TowerInRange`)
    (`KismetSystemLibrary.PrintString` (`KismetSystemLibrary.GetDisplayName` _array_element) true true (struct :`G` 0.66 :`B` 1.0 :`A` 1.0) 0.1)))

(event `self.StaticMesh.OnComponentBeginOverlap`
  (params (OverlappedComponent :type "PrimitiveComponent Object Reference") (OtherActor :type "Actor Object Reference") (OtherComp :type "PrimitiveComponent Object Reference") (OtherBodyIndex :type Integer) (bFromSweep :type Boolean) (SweepResult :type "HitResult Structure (by ref)"))
  (if (`self.ActorHasTag` OtherActor "obstaculo")
    (`KismetArrayLibrary.Array_AddUnique` (`self.TowerInRange`) OtherActor)
    (`PrimitiveComponent.SetMaterial` (`self.StaticMesh`) 0 "/Game/TowerD/Blueprints/MI_Red.MI_Red")))

(event `self.StaticMesh.OnComponentEndOverlap`
  (params (OverlappedComponent :type "PrimitiveComponent Object Reference") (OtherActor :type "Actor Object Reference") (OtherComp :type "PrimitiveComponent Object Reference") (OtherBodyIndex :type Integer))
  (bind _towerinrange (`self.TowerInRange`))
  (`KismetArrayLibrary.Array_RemoveItem` _towerinrange OtherActor)
  (if (`KismetArrayLibrary.Array_IsEmpty` _towerinrange)
    (`PrimitiveComponent.SetMaterial` (`self.StaticMesh`) 0 "/Game/TowerD/Blueprints/MI_Green.MI_Green")))

(fn `UserConstructionScript`
  (`parent.UserConstructionScript`)
  (`StaticMeshComponent.SetStaticMesh` (`self.StaticMesh`) (`self.Mesh`)))