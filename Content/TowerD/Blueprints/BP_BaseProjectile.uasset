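; BP_BaseProjectile is a homing projectile in the TowerD game that flies toward an assigned target component and damages it.
; The construction script passes the HomingTarget component to ProjectileMovement as its homing target.
; When the static mesh overlaps that exact component, it applies its Damage to the owning actor with the instigator's controller, then destroys itself, ignoring all other overlaps.
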(event `self.StaticMesh.OnComponentBeginOverlap`
  (params (OverlappedComponent :type "PrimitiveComponent Object Reference") (OtherActor :type "Actor Object Reference") (OtherComp :type "PrimitiveComponent Object Reference") (OtherBodyIndex :type Integer) (bFromSweep :type Boolean) (SweepResult :type "HitResult Structure (by ref)"))
  (if (== OtherComp (`self.HomingTarget`))
    (`GameplayStatics.ApplyDamage` OtherActor (`self.Damage`) (`self.GetInstigatorController`) self)
    (`self.K2_DestroyActor`)))

(fn `UserConstructionScript`
  (set `ProjectileMovementComponent.HomingTargetComponent` (`self.HomingTarget`) (`self.ProjectileMovement`)))