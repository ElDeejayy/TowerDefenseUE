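; Base tower for a tower defense game that fires homing projectiles at enemies inside its range sphere, sized from Radius on construction.
; Overlaps maintain EnemiesInRange and start, unpause or pause a looping attack-speed timer as enemies come and go.
; Shoot spawns a projectile homing on the first array entry, passing along Damage.
; Also provides a green ghost-material mode and a distance-to-goal sort, which is not called here.
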(event `SetGhostMode`
  (`PrimitiveComponent.SetMaterial` (`self.StaticMesh`) 0 "/Game/TowerD/Blueprints/MI_Green.MI_Green"))

(event `self.Sphere.OnComponentBeginOverlap`
  (params (OverlappedComponent :type "PrimitiveComponent Object Reference") (OtherActor :type "Actor Object Reference") (OtherComp :type "PrimitiveComponent Object Reference") (OtherBodyIndex :type Integer) (bFromSweep :type Boolean) (SweepResult :type "HitResult Structure (by ref)"))
  (`self.EnemyEnter` OtherActor))

(event `Shoot`
  (`|SpawnActorFromClass` "/Game/TowerD/Blueprints/BP_BaseProjectile.BP_BaseProjectile_C" (`SceneComponent.K2_GetComponentToWorld` (`self.Sphere`)) "Undefined" "MultiplyWithRoot" self (`Character.CapsuleComponent` (`|GetArrayItem` (`self.EnemiesInRange`))) (`self.Damage`) self))

(event `self.Sphere.OnComponentEndOverlap`
  (params (OverlappedComponent :type "PrimitiveComponent Object Reference") (OtherActor :type "Actor Object Reference") (OtherComp :type "PrimitiveComponent Object Reference") (OtherBodyIndex :type Integer))
  (`self.EnemyExit` OtherActor))

(fn `EnemyEnter`
  (params (Object :type "Object Object Reference"))
  (returns (Valid :type Boolean))
  (bind _asbp_base_enemy (cast `/Game/TowerD/Blueprints/BP_BaseEnemy` Object)
    (:`then`
      (`KismetArrayLibrary.Array_AddUnique` (`self.EnemiesInRange`) _asbp_base_enemy)
      (if (`KismetSystemLibrary.K2_IsValidTimerHandle` (`self.ShootTimerHandle`))
        (if (not (`KismetSystemLibrary.K2_IsTimerActiveHandle` (`self.ShootTimerHandle`)))
          (`KismetSystemLibrary.K2_UnPauseTimerHandle` (`self.ShootTimerHandle`)))
        (else
          (bind _returnvalue (`KismetSystemLibrary.K2_SetTimerDelegate` (`|CreateDelegate` :!event `Shoot`) (/ 1.0 (`self.VelocidadAtaque`)) true true))
          (set `self.ShootTimerHandle` _returnvalue)))
      (return true))
    (:`CastFailed`
      (return false))))

(fn `EnemyExit`
  (params (Object :type "Object Object Reference"))
  (returns (Empty :type Boolean))
  (bind _enemiesinrange (`self.EnemiesInRange`))
  (bind _asbp_base_enemy (cast `/Game/TowerD/Blueprints/BP_BaseEnemy` Object))
  (`KismetArrayLibrary.Array_RemoveItem` _enemiesinrange _asbp_base_enemy)
  (if (`KismetArrayLibrary.Array_IsEmpty` _enemiesinrange)
    (`KismetSystemLibrary.K2_PauseTimerHandle` (`self.ShootTimerHandle`))
    (return true)
    (else
      (return false))))

(fn `OrderEnemiesByDistance`
  (locals (Distances :type "Array of Float (double-precision)") (`Distances Sorted` :type "Array of Float (double-precision)") (`Local Enemies` :type "Array of /Game/TowerD/Blueprints/BP_BaseEnemy Object Reference"))
  (for _array_element (`self.EnemiesInRange`)
    (`/Engine/EditorBlueprintResources/StandardMacros.IsValid` _array_element
      (:`Is Valid`
        (`KismetArrayLibrary.Array_Add` (`local.Distances`) (`/Game/TowerD/Blueprints/BP_BaseEnemy.Distance to goal location` _array_element))
        (`KismetArrayLibrary.Array_Add` (`local.Local Enemies`) _array_element))))
  (bind _output_get (set `local.Distances Sorted` (`local.Distances`)))
  (`KismetArrayLibrary.SortFloatArray` _output_get)
  (`KismetArrayLibrary.Array_Clear` (`self.EnemiesInRange`))
  (for _array_element_2 _output_get
    (`KismetArrayLibrary.Array_Add` (`self.EnemiesInRange`) (`|GetArrayItem` (`local.Local Enemies`) (`KismetArrayLibrary.Array_Find` (`local.Distances`) _array_element_2)))))

(fn `UserConstructionScript`
  (`SphereComponent.SetSphereRadius` (`self.Sphere`) (`self.Radius`) true))