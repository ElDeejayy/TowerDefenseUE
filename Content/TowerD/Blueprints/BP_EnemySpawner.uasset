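; Tower defense enemy spawner that releases each round's enemies in sequential groups when the game mode signals round start.
; SpawnerData, indexed by the game mode's current round (RondaActual), gives each group's enemy type, count, spawn rate and delay.
; A looping timer spawns enemies at the spawner, passing them the Destination location and game mode.
; Full groups advance to the next; after the last, it resets and notifies the game mode that spawning finished.
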(event `self.ReceiveBeginPlay`
  (bind _asgm_tower_defense (cast `/Game/TowerD/Game/GM_TowerDefense` (`GameplayStatics.GetGameMode`)))
  (bind _output_get (set `self.As GM Tower Defense` _asgm_tower_defense))
  (add `/Game/TowerD/Game/GM_TowerDefense.RoundStart` _output_get (delegate `RoundStart_Event`)))

(event `Spawn`
  (if (>= (`self.EnemiesSpawnedinCurrentGroup`) (`self.GetNumEnemies`))
    (`KismetSystemLibrary.K2_ClearAndInvalidateTimerHandle` (`self.RotateTimerHandle`))
    (`/Engine/EditorBlueprintResources/StandardMacros.IncrementInt` (`self.CurrentGroup`)
      (:`  `
        (set `self.EnemiesSpawnedinCurrentGroup` 0)
        (`self.StartNewGroup`)))
    (else
      (`|SpawnActorFromClass` (`self.GetEnemyType`) (`self.GetTransform`) "AdjustIfPossibleButAlwaysSpawn" "MultiplyWithRoot" null (`SceneComponent.K2_GetComponentLocation` (`self.Destination`)) (`self.As GM Tower Defense`) null)
      (`/Engine/EditorBlueprintResources/StandardMacros.IncrementInt` (`self.EnemiesSpawnedinCurrentGroup`)))))

(event `RoundStart_Event`
  (`self.StartNewGroup`))

(event `StartNewGroup`
  (bind _currentgroup (`self.CurrentGroup`))
  (bind _output_membervar_0 (break `/Game/TowerD/Blueprints/S_EnemyRoundData` (`|GetArrayItem` (`self.SpawnerData`) (`/Game/TowerD/Game/GM_TowerDefense.RondaActual` (`self.As GM Tower Defense`)))))
  (`KismetSystemLibrary.PrintString` (`KismetStringLibrary.Conv_IntToString` _currentgroup))
  (if (`KismetArrayLibrary.Array_IsValidIndex` _output_membervar_0 _currentgroup)
    (bind _returnvalue (`KismetSystemLibrary.K2_SetTimerDelegate` (delegate `Spawn`) (`self.GetSpawnRate`) true true (`self.GetGroupDelay`)))
    (set `self.RotateTimerHandle` _returnvalue)
    (else
      (set `self.CurrentGroup` 0)
      (`/Game/TowerD/Game/GM_TowerDefense.SetSpawningFinished` (`self.As GM Tower Defense`)))))

(fn `GetEnemyType`
  (returns (EnemyType :type "/Game/TowerD/Blueprints/BP_BaseEnemy Class Reference"))
  (bind _output_membervar_0 (break `/Game/TowerD/Blueprints/S_EnemyRoundData` (`|GetArrayItem` (`self.SpawnerData`) (`/Game/TowerD/Game/GM_TowerDefense.RondaActual` (`self.As GM Tower Defense`)))))
  (return (`.EnemyType_8_9BC22077492FA96F355593A2A75FE3EE` (break `/Game/TowerD/Structures+Enumerators/S_EnemySpawnerData` (`|GetArrayItem` _output_membervar_0 (`self.CurrentGroup`))))))

(fn `GetGroupDelay`
  (returns (GroupDelay :type "Float (double-precision)"))
  (bind _output_membervar_0 (break `/Game/TowerD/Blueprints/S_EnemyRoundData` (`|GetArrayItem` (`self.SpawnerData`) (`/Game/TowerD/Game/GM_TowerDefense.RondaActual` (`self.As GM Tower Defense`)))))
  (return (`.GroupDelay_11_D67031604FF0EA1D8FD495B8BC61EA94` (break `/Game/TowerD/Structures+Enumerators/S_EnemySpawnerData` (`|GetArrayItem` _output_membervar_0 (`self.CurrentGroup`))))))

(fn `GetNumEnemies`
  (returns (NumEnemies :type Integer))
  (bind _output_membervar_0 (break `/Game/TowerD/Blueprints/S_EnemyRoundData` (`|GetArrayItem` (`self.SpawnerData`) (`/Game/TowerD/Game/GM_TowerDefense.RondaActual` (`self.As GM Tower Defense`)))))
  (return (`.NumEnemies_2_B8C5DB9A4109E7D0F859A6985CC640B0` (break `/Game/TowerD/Structures+Enumerators/S_EnemySpawnerData` (`|GetArrayItem` _output_membervar_0 (`self.CurrentGroup`))))))

(fn `GetSpawnRate`
  (returns (GroupDelay :type "Float (double-precision)"))
  (bind _output_membervar_0 (break `/Game/TowerD/Blueprints/S_EnemyRoundData` (`|GetArrayItem` (`self.SpawnerData`) (`/Game/TowerD/Game/GM_TowerDefense.RondaActual` (`self.As GM Tower Defense`)))))
  (return (`.SpawnRate_5_513071E54260F544AAB0A48659639412` (break `/Game/TowerD/Structures+Enumerators/S_EnemySpawnerData` (`|GetArrayItem` _output_membervar_0 (`self.CurrentGroup`))))))

(fn `UserConstructionScript`)