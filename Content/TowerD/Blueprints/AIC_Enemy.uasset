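; AI controller for tower defense enemies that walks its pawn to a goal location.
; On possess it caches the pawn as a BP_BaseEnemy, and its MoveToGoalLocation event runs an AI MoveTo toward the given destination.
; On arrival it passes that enemy to the game mode's RestarVidaJugador to subtract player life, then destroys the controller itself.
; A failed move only prints a debug message.
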(event `MoveToGoalLocation`
  (params (Destination :type "Vector Structure"))
  (bind _movementresult (`|AIMoveTo` (`self.K2_GetPawn`) Destination null)
    (:`OnSuccess`
      (bind _asgm_tower_defense (cast `/Game/TowerD/Game/GM_TowerDefense` (`GameplayStatics.GetGameMode`)))
      (`/Game/TowerD/Game/GM_TowerDefense.RestarVidaJugador` _asgm_tower_defense (`self.As BP Base Enemy`))
      (`self.K2_DestroyActor`))
    (:`OnFail`
      (`KismetSystemLibrary.PrintString` (`KismetStringLibrary.Concat_StrStr` "Movement failed on" (`KismetSystemLibrary.GetDisplayName` (`self.K2_GetPawn`)) "Cause" (`|GetEnumeratorNameAsString` _movementresult))))))

(event `self.ReceivePossess`
  (params (PossessedPawn :type "Pawn Object Reference"))
  (bind _asbp_base_enemy (cast `/Game/TowerD/Blueprints/BP_BaseEnemy` PossessedPawn))
  (set `self.As BP Base Enemy` _asbp_base_enemy))

(fn `UserConstructionScript`)