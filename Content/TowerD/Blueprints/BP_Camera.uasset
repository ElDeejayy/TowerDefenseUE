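; BP_Camera is the possessable camera for the tower defense game, passing left mouse clicks on to the game mode to build towers.
; On BeginPlay it caches GM_TowerDefense and registers itself as that game mode's Camera.
; On possession it prints the controller's name and enables input from player controller 0.
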(event `self.ReceivePossessed`
  (params (NewController :type "Controller Object Reference"))
  (`KismetSystemLibrary.PrintString` (`KismetSystemLibrary.GetDisplayName` NewController))
  (`self.EnableInput` (`GameplayStatics.GetPlayerController` 0)))

(event `Key|LeftMouseButton`
  (params (Key :type "Key Structure"))
  (:`Pressed`
    (`/Game/TowerD/Game/GM_TowerDefense.Build Tower` (`self.As GM Tower Defense`))))

(event `self.ReceiveBeginPlay`
  (bind _asgm_tower_defense (cast `/Game/TowerD/Game/GM_TowerDefense` (`GameplayStatics.GetGameMode`)))
  (bind _output_get (set `self.As GM Tower Defense` _asgm_tower_defense))
  (set `/Game/TowerD/Game/GM_TowerDefense.Camera` self _output_get))

(fn `UserConstructionScript`)