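; BP_BaseEnemy is the tower defense base enemy, walking to a destination via its AIC_Enemy controller once possessed.
; Damage lowers HP, death pays a money reward, and spawn and destruction are reported to the game mode.
; Freeze divides walk speed and swaps materials, using a retriggerable delay to extend the effect without stacking.
; A path-cost distance-to-goal update exists, but its timer setup is unconnected.
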(event `UpdateCurrentDistanceToGoalLocation`
  (bind _returnvalue (`NavigationSystemV1.FindPathToLocationSynchronously` (`self.K2_GetActorLocation`) (`self.Destination`) (`self.As AIC Enemy`) "/Game/TowerD/Navigation/BP_EnemyNavFilter.BP_EnemyNavFilter_C"))
  (set `self.Distance to goal location` (`NavigationPath.GetPathCost` _returnvalue)))

(event `self.ReceiveBeginPlay`
  (`/Game/TowerD/Game/GM_TowerDefense.EnemySpawned` (`self.GameMode`)))

(event `self.ReceiveAnyDamage`
  (params (Damage :type "Float (single-precision)") (DamageType :type "DamageType Object Reference") (InstigatedBy :type "Controller Object Reference") (DamageCauser :type "Actor Object Reference"))
  (bind _output_get (set `self.CurrentHp` (- (`self.CurrentHp`) Damage)))
  (if (<= _output_get 0.0)
    (`/Game/TowerD/Game/GM_TowerDefense.MoneyReward` (`self.GameMode`) (`self.RecompensaDinero`))
    (`self.K2_DestroyActor`)))

(event `self.ReceivePossessed`
  (params (NewController :type "Controller Object Reference"))
  ; Comprueba que cuando entra vea si es de ese tipo. Si lo es, sigue,sino "cast failed"
  (bind _asaic_enemy (cast `/Game/TowerD/Blueprints/AIC_Enemy` NewController))
  (set `self.As AIC Enemy` _asaic_enemy)
  (`KismetSystemLibrary.DelayUntilNextTick`)
  (`/Game/TowerD/Blueprints/AIC_Enemy.MoveToGoalLocation` (`self.As AIC Enemy`) (`self.Destination`)))

(event `Freeze`
  (params (Duration :type "Float (single-precision)") (`Slow Amount` :type "Float (double-precision)"))
  (bind _charactermovement (`self.CharacterMovement`))
  (bind _mesh (`self.Mesh`))
  (bind _charactermovement_2 (`self.CharacterMovement`))
  (bind _mesh_2 (`self.Mesh`))
  (if (not (`self.Feezed`))
    (set `self.Feezed` true)
    (set `CharacterMovementComponent.MaxWalkSpeed` (/ (`CharacterMovementComponent.MaxWalkSpeed` _charactermovement_2) `Slow Amount`) _charactermovement_2)
    (`PrimitiveComponent.SetMaterial` _mesh_2 0 "/Game/TowerD/Art/Animations/MI_Ch_49_body1_Freeze.MI_Ch_49_body1_Freeze")
    (`PrimitiveComponent.SetMaterial` _mesh_2 1 "/Game/TowerD/Art/Animations/MI_Ch_49_body1_Freeze.MI_Ch_49_body1_Freeze"))
  (`KismetSystemLibrary.RetriggerableDelay` Duration)
  (set `CharacterMovementComponent.MaxWalkSpeed` (* (`CharacterMovementComponent.MaxWalkSpeed` _charactermovement) `Slow Amount`) _charactermovement)
  (`PrimitiveComponent.SetMaterial` _mesh 0 "/Game/TowerD/Art/Animations/Ch_49_body1.Ch_49_body1")
  (`PrimitiveComponent.SetMaterial` _mesh 1 "/Game/TowerD/Art/Animations/Ch_49_body2.Ch_49_body2")
  (set `self.Feezed` false))

(event `self.ReceiveDestroyed`
  (`/Game/TowerD/Game/GM_TowerDefense.EnemyDead` (`self.GameMode`)))

(fn `UserConstructionScript`
  (set `self.CurrentHp` (`self.MaxHP`)))