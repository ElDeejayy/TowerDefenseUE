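; Tower defense game mode that runs rounds, player money and health, tower placement, and win or loss handling.
; Placement spawns a preview actor that a looping timer moves to follow the cursor; building spawns the chosen tower and deducts its price.
; Enemy spawn and death counters trigger round end or the victory widget on the final round.
; A separate check shows the defeat screen, while victory-check and spawning-finished functions are empty.
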(event `TowerPlacementMode`
  (params (Tower :type "/Game/TowerD/Blueprints/BP_BaseTower Class Reference"))
  (bind _output_get (set `self.CurrentTowerToPlaceClass` Tower))
  (bind _returnvalue (`|SpawnActorFromClass` "/Game/TowerD/Blueprints/BP_Preview_Tower.BP_Preview_Tower_C" (`KismetMathLibrary.MakeTransform` (`.Location` (`GameplayStatics.BreakHitResult` (`PlayerController.GetHitResultUnderCursorForObjects` (`GameplayStatics.GetPlayerController` 0) (`|MakeArray` "ObjectTypeQuery1" :!type "EObjectTypeQuery Enum") true)))) "Undefined" "MultiplyWithRoot" null (`.Mesh` (defaults `Object` _output_get)) null))
  (set `self.CurrentTowerPreview` _returnvalue)
  (bind _returnvalue_2 (`KismetSystemLibrary.K2_SetTimerDelegate` (delegate `UpdateTowerPosition`) 0.001 true))
  (set `self.TowerTimerHandle` _returnvalue_2))

(event `UpdateTowerPosition`
  (`self.K2_SetActorLocation` (`self.CurrentTowerPreview`) (`.Location` (`GameplayStatics.BreakHitResult` (`PlayerController.GetHitResultUnderCursorByChannel` (`GameplayStatics.GetPlayerController` 0) "TraceTypeQuery1" true))) false true))

(event `StartRound`
  (`/Engine/EditorBlueprintResources/StandardMacros.IncrementInt` (`self.RondaActual`)
    (:`  `
      (`self.RoundStart`))))

(event `self.ReceiveBeginPlay`
  (bind _returnvalue (`GameplayStatics.GetPlayerController` 0))
  (set `PlayerController.bShowMouseCursor` true _returnvalue)
  (`WidgetBlueprintLibrary.SetInputMode_GameAndUIEx` _returnvalue null "DoNotLock" false)
  (bind _returnvalue_2 (`|CreateWidget` "/Game/TowerD/Blueprints/WBP_Interface.WBP_Interface_C" null self))
  (`UserWidget.AddToViewport` _returnvalue_2 0))

(fn `Build Tower`
  (bind _currenttowerpreview (`self.CurrentTowerPreview`)
    (:`then`
      (`|SpawnActorFromClass` (`self.CurrentTowerToPlaceClass`) (`KismetMathLibrary.MakeTransform` (`self.K2_GetActorLocation` _currenttowerpreview)) "AdjustIfPossibleButAlwaysSpawn" "MultiplyWithRoot" null null)
      (`KismetSystemLibrary.K2_PauseTimerHandle` (`self.TowerTimerHandle`))
      (`self.SpendMoney` (`.Price` (defaults `Object` (`self.CurrentTowerToPlaceClass`))))
      (`self.K2_DestroyActor` (`self.CurrentTowerPreview`))
      (set `self.CurrentTowerPreview` null)
      (set `self.CurrentTowerToPlaceClass` null))
    (:`else`)))

(fn `CheckGameOver`
  (bind _output_get (set `self.Vida Jugador` (`self.VidaJugador`)))
  (if (<= _output_get 0)
    (bind _returnvalue (`|CreateWidget` "/Game/TowerD/Blueprints/WBP_Defeat.WBP_Defeat_C"))
    (`UserWidget.AddToViewport` _returnvalue 0)))

(fn `CheckVictory`)

(fn `EnemyDead`
  (bind _result (`/Engine/EditorBlueprintResources/StandardMacros.DecrementInt` (`self.NumEnemigos`))
    (:`  `
      (if (and (<= _result 0) (`self.SpawningFinished`))
        (if (== (`self.RondaFinal`) (`self.RondaActual`))
          (bind _returnvalue (`|CreateWidget` "/Game/TowerD/Blueprints/WBP_Victory.WBP_Victory_C"))
          (`UserWidget.AddToViewport` _returnvalue 0)
          (else
            (`self.RoundEnded`)))))))

(fn `EnemySpawned`
  (`/Engine/EditorBlueprintResources/StandardMacros.IncrementInt` (`self.NumEnemigos`)))

(fn `RestarVidaJugador`
  (params (Enemy :type "/Game/TowerD/Blueprints/BP_BaseEnemy Object Reference"))
  (bind _output_get (set `self.VidaJugador` (- (`self.VidaJugador`) (`/Game/TowerD/Blueprints/BP_BaseEnemy.DanoAlJugador` Enemy))))
  (if (<= _output_get 0)
    (`KismetSystemLibrary.PrintString` "Bye bye")
    (return)
    (else
      (`self.K2_DestroyActor` (`local.Enemy`)))))

(fn `SetSpawningFinished`)

(fn `SpendMoney`
  (params (Amount :type Integer))
  (set `self.Dinero` (- (`self.Dinero`) Amount)))

(fn `UserConstructionScript`)